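; BP_BulletTrail is a test actor that previews a bullet trail effect on a fake moving bullet.
; On BeginPlay, the FakeMovement timeline sweeps the actor along negative world X each update.
; Each update also activates the BulletTrail FX and sets its lifetime (fixed at zero), current bullet position and trail end.
; Trail end is movement direction scaled by TrailDistance, a test stand-in for a fixed target location fed once.
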(event EventBeginPlay
  (bind _bullettrail (Variables|Default|GetBulletTrail))
  ;[0.15 0.15 0.15 0.5] For testing only.
  (Timeline|FakeMovement PlayFromStart
    (:Update
      (Variables|Default|SetLastPosition (Transformation|GetActorLocation))
      (Transformation|AddActorWorldOffset (Math|Vector|MakeVector -1.0 0.0 0.0) true)
      ;[0.15 0.15 0.15 0.5] Plugin the lifetime of the bullet/time left of the bullet before it reaches the catching location
      (Effects|Components|ParticleSystem|SetFloatParameter (Variables|Default|GetBulletTrail) "BulletLifetime" 0.0)
      ;[0.15 0.15 0.15 0.5] Activates the FX
      (Components|Activation|Activate (Variables|Default|GetBulletTrail) true)
      ;[0.15 0.15 0.15 0.5] For testing purposes only. We'll need to feed the target location once here. The value must not change or the trail will expand beyond the target location.
      (Effects|Components|ParticleSystem|SetVectorParameter _bullettrail "BulletTrailEnd" (* (Variables|Default|GetTrailDistance) (Math|Vector|Normalize (- (Transformation|GetActorLocation) (Variables|Default|GetLastPosition)))))
      ;[0.15 0.15 0.15 0.5] Feed the bullet position when it's moving
      (Effects|Components|ParticleSystem|SetVectorParameter _bullettrail "Bullet" (Transformation|GetActorLocation)))))

(fn ConstructionScript)