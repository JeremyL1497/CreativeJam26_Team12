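; Blood puddle spawner actor that keeps adding BP_BloodPuddle actors around itself until a cap is reached.
; A looping one-second timer started on BeginPlay counts every puddle in the level, so the MaxBLood limit is global rather than per spawner.
; The check compares last index to the limit, allowing one puddle above MaxBLood.
; Each puddle spawns at a random horizontal offset scaled by the Sphere component's radius, at a fixed world height.
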(event Custom|Timer
  (bind _returnvalue (Transformation|GetActorLocation))
  (bind _returnvalue_2 (Math|Random|RandomUnitVector))
  (bind _sphere (Variables|Default|GetSphere))
  (bind _sphereradius (Collision|GetComponentBounds _sphere))
  (bind _returnvalue_3 (Math|Vector|MakeVector (.x _returnvalue_2) (.y _returnvalue_2) 0.0))
  (bind _returnvalue_4 (Math|Random|RandomFloatinRange 25.0 _sphereradius))
  (bind _returnvalue_5 (* _returnvalue_3 _returnvalue_4))
  (bind _returnvalue_6 (+ _returnvalue_5 _returnvalue))
  (bind (_x _y) (Math|Vector|BreakVector _returnvalue_6))
  (bind _outactors (Actor|GetAllActorsOfClass "/Game/Blueprints/BP_BloodPuddle.BP_BloodPuddle_C"))
  (if (< (Utilities|Array|LastIndex _outactors) (Variables|Default|GetMaxBLood))
    (Game|SpawnActorfromClass "/Game/Blueprints/BP_BloodPuddle.BP_BloodPuddle_C" (Math|Transform|MakeTransform (Math|Vector|MakeVector _x _y 4e+01) "0, 0, 0" "1.000000,1.000000,1.000000") "Undefined" "MultiplyWithRoot" 0 0)))

(event EventBeginPlay
  (bind _returnvalue (Utilities|Time|SetTimerbyEvent (delegate Custom|Timer) 1.0 true))
  (Utilities|Time|UnpauseTimerbyHandle _returnvalue))

(event Collision|EventActorBeginOverlap
  (params (OtherActor :type Actor%20Object%20Reference)))

(event EventTick
  (params (DeltaSeconds :type Float%20%28single-precision%29)))

(fn ConstructionScript)