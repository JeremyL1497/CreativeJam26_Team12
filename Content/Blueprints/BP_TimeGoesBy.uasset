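; BP_TimeGoesBy is an actor that shows a Niagara blood effect while something overlaps its Sphere.
; Overlap begin adds the Niagara component above the actor, stores it as BloodFX and activates it; overlap end deactivates and destroys it.
; While BloodFX is valid, Tick passes the actor's location to its BloodPuddlePos parameter.
; Overlaps are unfiltered and share one BloodFX reference, so each new overlap overwrites the previous one.
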(event OnComponentBeginOverlap(Sphere)
  (params (OverlappedComponent :type Primitive%20Component%20Object%20Reference) (OtherActor :type Actor%20Object%20Reference) (OtherComp :type Primitive%20Component%20Object%20Reference) (OtherBodyIndex :type Integer) (bFromSweep :type Boolean) (SweepResult :type Hit%20Result%20Structure%20%28by%20ref%29))
  (bind _returnvalue (AddComponent|AddNiagaraComponent false (Math|Transform|MakeTransform "0.000000,0.000000,100.000000" "0, 0, 0" "1.000000,1.000000,1.000000")))
  (bind _output_get (Variables|Default|SetBloodFX _returnvalue))
  (Components|Activation|Activate _output_get false))

(event OnComponentEndOverlap(Sphere)
  (params (OverlappedComponent :type Primitive%20Component%20Object%20Reference) (OtherActor :type Actor%20Object%20Reference) (OtherComp :type Primitive%20Component%20Object%20Reference) (OtherBodyIndex :type Integer))
  (bind _bloodfx (Variables|Default|GetBloodFX))
  (Components|Activation|Deactivate _bloodfx)
  (Components|DestroyComponent _bloodfx))

(event EventBeginPlay)

(event Collision|EventActorBeginOverlap
  (params (OtherActor :type Actor%20Object%20Reference)))

(event EventTick
  (params (DeltaSeconds :type Float%20%28single-precision%29))
  (bind _bloodfx (Variables|Default|GetBloodFX)
    (:then
      (Effects|Components|ParticleSystem|SetVectorParameter _bloodfx "BloodPuddlePos" (Transformation|GetActorLocation)))
    (:else)))

(fn ConstructionScript)