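; Blood puddle actor that gets consumed once something overlaps its sphere, then removes itself.
; The overlap adds and activates a Niagara effect, fed the puddle's position every tick, and plays a timeline that rescales the cube.
; When the timeline finishes, the effect deactivates and the actor destroys itself once the particle system finishes.
; Ending the overlap does not stop consumption.
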(event OnComponentBeginOverlap(Sphere)
  (params (OverlappedComponent :type Primitive%20Component%20Object%20Reference) (OtherActor :type Actor%20Object%20Reference) (OtherComp :type Primitive%20Component%20Object%20Reference) (OtherBodyIndex :type Integer) (bFromSweep :type Boolean) (SweepResult :type Hit%20Result%20Structure%20%28by%20ref%29))
  (Variables|Default|GetBloodFX
    (:then
      _)
    (:else
      (bind _returnvalue (AddComponent|AddNiagaraComponent false))
      (bind _output_get (Variables|Default|SetBloodFX _returnvalue))))
  (Components|Activation|Activate _output_get false)
  (Audio|Components|Audio|Play (Variables|Default|GetConsumingBlood)))

(event OnComponentEndOverlap(Sphere)
  (params (OverlappedComponent :type Primitive%20Component%20Object%20Reference) (OtherActor :type Actor%20Object%20Reference) (OtherComp :type Primitive%20Component%20Object%20Reference) (OtherBodyIndex :type Integer)))

(event Custom|BloodAllConsumed
  (bind _bloodfx (Variables|Default|GetBloodFX)
    (:then
      (EventDispatchers|AssignOnSystemFinished _bloodfx (delegate Custom|OnSystemFinished_Event)))
    (:else
      _))
  (Components|Activation|Deactivate _bloodfx))

(event Custom|OnSystemFinished_Event
  (params (PSystem :type Niagara%20Component%20Object%20Reference))
  (Actor|DestroyActor))

(event EventTick
  (params (DeltaSeconds :type Float%20%28single-precision%29))
  (bind _bloodfx (Variables|Default|GetBloodFX)
    (:then
      (Effects|Components|ParticleSystem|SetVectorParameter _bloodfx "BloodPuddlePos" (Transformation|GetActorLocation)))
    (:else)))

(fn ConstructionScript)