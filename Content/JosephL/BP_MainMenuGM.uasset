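; Main menu game mode that runs a slow-motion bullet-capture tutorial with the MarcelDemon actor.
; BeginPlay switches the view to a CineCameraActor and slows global time while offsetting player dilation to keep normal speed.
; The demon fires three angled tutorial bullets, polling capture counts before the second and third, then Stage1 restores normal time.
; A separate DemonShoot event, uncalled here, fires base bullets at random yaw.
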(event Custom|DemonShoot
  (bind _returnvalue (Game|SpawnActorfromClass "/Game/Marcel/MarcelBaseBullet.MarcelBaseBullet_C" (Math|Transform|MakeTransform (Variables|Default|GetDemonAimTransform) (Math|Rotator|MakeRotator 0.0 0.0 (Math|Random|RandomFloatinRange -55.0 55.0)) "1.000000,1.000000,1.000000") "AlwaysSpawn" "MultiplyWithRoot" 0 0))
  (Development|PrintString (Utilities|GetDisplayName _returnvalue)))

(event Custom|Tutorialization
  ;[0.15 0.15 0.15 0.5] TUTORIAL
  (if (== (Variables|Default|GetStage) 0)
    (CallFunction|TutorialDemonShoot)
    (Utilities|Time|SetGlobalTimeDilation 0.67)
    (Variables|/Script/Engine.Actor|SetCustomTimeDilation (Game|GetPlayerCharacter 0) (/ 1.0 (Class|GameplayStatics|GetGlobalTimeDilation)))
    (elif (== (Variables|Default|GetStage) 1)
      (CallFunction|Stage1))))

(event Custom|TutorialDemonShoot
  ;[0.15 0.15 0.15 0.5] TUTORIAL
  (if (and (== (Variables|Default|GetTutorialBulletsFired) 0) (== (Variables|Default|GetTutorialBulletsCaptured) 0))
    (Game|SpawnActorfromClass "/Game/Marcel/MarcelTutorialBullet.MarcelTutorialBullet_C" (Math|Transform|MakeTransform (Variables|Default|GetDemonAimTransform) "0.000000,14.000000,0.000000" "1.000000,1.000000,1.000000") "AlwaysSpawn" "MultiplyWithRoot" 0 0)
    (Utilities|FlowControl|Delay 1.0)
    (Math|Integer|IncrementInt (Variables|Default|GetTutorialBulletsFired)
      (:%20%20
        (if (and (== (Variables|Default|GetTutorialBulletsFired) 1) (== (Variables|Default|GetTutorialBulletsCaptured) 1)) :!label _label
          (Game|SpawnActorfromClass "/Game/Marcel/MarcelTutorialBullet.MarcelTutorialBullet_C" (Math|Transform|MakeTransform (Variables|Default|GetDemonAimTransform) "0.000000,-25.000000,0.000000" "1.000000,1.000000,1.000000") "AlwaysSpawn" "MultiplyWithRoot" 0 0)
          (Utilities|FlowControl|Delay 1.0)
          (Math|Integer|IncrementInt (Variables|Default|GetTutorialBulletsFired)
            (:%20%20
              (if (and (== (Variables|Default|GetTutorialBulletsFired) 2) (== (Variables|Default|GetTutorialBulletsCaptured) 2)) :!label _label_2
                (Game|SpawnActorfromClass "/Game/Marcel/MarcelTutorialBullet.MarcelTutorialBullet_C" (Math|Transform|MakeTransform (Variables|Default|GetDemonAimTransform) "0.000000,48.000000,0.000000" "1.000000,1.000000,1.000000") "AlwaysSpawn" "MultiplyWithRoot" 0 0)
                (Utilities|FlowControl|Delay 1.0)
                (Math|Integer|IncrementInt (Variables|Default|GetTutorialBulletsFired)
                  (:%20%20
                    (Utilities|FlowControl|Delay 2.0)
                    (Math|Integer|IncrementInt (Variables|Default|GetStage)
                      (:%20%20
                        (CallFunction|Stage1)))))
                (else
                  (Utilities|FlowControl|Delay 0.5)
                  (goto _label_2)))))
          (else
            (Utilities|FlowControl|Delay 0.5)
            (goto _label)))))))

(event Custom|Stage1
  (Development|PrintString "Stage 1")
  (if (== (Variables|Default|GetStage) 1)
    (Utilities|Time|SetGlobalTimeDilation 1.0)
    (Variables|/Script/Engine.Actor|SetCustomTimeDilation (Game|GetPlayerCharacter 0) 1.0)))

(event EventBeginPlay
  ;[0.15 0.15 0.15 0.5] Declare Variables
  (Variables|Default|SetStage 0)
  (bind _returnvalue (Actor|GetActorOfClass "/Script/CinematicCamera.CineCameraActor"))
  (bind _output_get (Variables|Default|SetCamera _returnvalue))
  (Game|Player|SetViewTargetwithBlend (Game|GetPlayerController 0) _output_get 0.0 "VTBlend_Linear" 0.0 false)
  (bind _returnvalue_2 (Actor|GetActorOfClass "/Game/Marcel/MarcelDemon.MarcelDemon_C"))
  (bind _output_get_2 (Variables|Default|SetDemon _returnvalue_2))
  (Variables|Default|SetDemonAimTransform (Math|Vector|MakeVector (+ (.X (Math|Vector|BreakVector (.location (Transformation|GetActorTransform _output_get_2)))) 1e+02) (.Y (Math|Vector|BreakVector (.location (Transformation|GetActorTransform _output_get_2)))) (.Z (Math|Vector|BreakVector (.location (Transformation|GetActorTransform _output_get_2))))))
  (CallFunction|Tutorialization))

(fn ConstructionScript)