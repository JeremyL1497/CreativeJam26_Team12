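; Demon bullet projectile that the player can either catch or be hit by.
; Tick moves it along its forward vector, with a timeline curve blending speed between max and min velocity.
; Overlapping the player's reach radius shows a widget and registers it as catchable, while capsule contact removes about a third of health and destroys it.
; ExecuteCatch increments the game mode's capture count and destroys the bullet; trail FX nodes are left unconnected.
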(event OnComponentBeginOverlap(Box)
  (params (OverlappedComponent :type Primitive%20Component%20Object%20Reference) (OtherActor :type Actor%20Object%20Reference) (OtherComp :type Primitive%20Component%20Object%20Reference) (OtherBodyIndex :type Integer) (bFromSweep :type Boolean) (SweepResult :type Hit%20Result%20Structure%20%28by%20ref%29))
  (bind _asbp_final_player (Utilities|Casting|CastToBP_FinalPlayer OtherActor))
  (if (== OtherComp (Variables|/Game/Final/BP_FinalPlayer.BP_FinalPlayer_C|GetReachRadius _asbp_final_player))
    (Development|PrintString "Reach")
    (Rendering|SetVisibility (Variables|Default|GetWidget) true false)
    (Variables|/Game/Final/BP_FinalPlayer.BP_FinalPlayer_C|SetCatchableBullet (.AsBP%20Final%20Player (Utilities|Casting|CastToBP_FinalPlayer (Game|GetPlayerCharacter 0))) self)
    (elif (== OtherComp (Variables|/Script/Engine.Character|GetCapsuleComponent _asbp_final_player))
      (Development|PrintString "Hit")
      (bind _output_get (Variables|/Game/Final/BP_FinalPlayer.BP_FinalPlayer_C|SetPlayerCurrentHealth _asbp_final_player (- (Variables|/Game/Final/BP_FinalPlayer.BP_FinalPlayer_C|GetPlayerCurrentHealth _asbp_final_player) 0.333334)))
      (Development|PrintString (Utilities|String|Append "Player Current Health: " (Utilities|String|ToString(Float) _output_get)) true false "(R=1.000000,G=0.209069,B=0.209069,A=1.000000)")
      (Actor|DestroyActor))))

(event OnComponentEndOverlap(Box)
  (params (OverlappedComponent :type Primitive%20Component%20Object%20Reference) (OtherActor :type Actor%20Object%20Reference) (OtherComp :type Primitive%20Component%20Object%20Reference) (OtherBodyIndex :type Integer))
  (bind _asbp_final_player (Utilities|Casting|CastToBP_FinalPlayer OtherActor))
  (if (== OtherComp (Variables|/Game/Final/BP_FinalPlayer.BP_FinalPlayer_C|GetReachRadius _asbp_final_player))
    (Rendering|SetVisibility (Variables|Default|GetWidget) false false)
    (Variables|/Game/Final/BP_FinalPlayer.BP_FinalPlayer_C|SetCatchableBullet (.AsBP%20Final%20Player (Utilities|Casting|CastToBP_FinalPlayer (Game|GetPlayerCharacter 0))) 0)))

(event EventBeginPlay
  (bind _alpha (Timeline|SpeedCurve_Timeline PlayFromStart)))

(event Collision|EventActorBeginOverlap
  (params (OtherActor :type Actor%20Object%20Reference))
  (|CallParentFunction OtherActor) ; This node is disabled and will not be called.\nDrag off pins to build functionality.
)

(event EventTick
  (params (DeltaSeconds :type Float%20%28single-precision%29))
  (Transformation|AddActorWorldOffset (* DeltaSeconds (Math|Float|Lerp (Variables|Default|GetMaxVelocity) (Variables|Default|GetMinVelocity) (stale EventBeginPlay _alpha)) (Transformation|GetActorForwardVector))))

(event EventExecuteCatch
  ;[0.15 0.15 0.15 0.5] Capture Success Logic
  (bind _result (Math|Integer|IncrementInt (Variables|/Game/Final/GM_Final.GM_Final_C|GetBulletsCaptured (.AsGM%20Final (Utilities|Casting|CastToGM_Final (Game|GetGameMode)))))
    (:%20%20
      (Development|PrintString (Utilities|String|Append (Utilities|String|ToString(Integer) _result) " bullet(s) captured"))
      (Actor|DestroyActor))))

(fn ConstructionScript
  (|CallParentFunction))