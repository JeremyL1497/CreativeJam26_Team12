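; Game mode for the final boss fight, running a bullet tutorial and then Stage 1.
; BeginPlay sets up the camera, the demon's aim point and full player health.
; The tutorial slows global time while keeping the player at normal speed, polling with Delay loops to fire each bullet after the previous capture.
; A boss tutorial QTE then leads into Stage 1's timed, random-yaw demon shots and pre-programmed QTE at normal speed.
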(event Custom|DemonShoot
  ;[0.15 0.15 0.15 0.5 90] DEMON SHOOT
  (bind _returnvalue (Game|SpawnActorfromClass "/Game/Final/BP_FinalBulletDemon.BP_FinalBulletDemon_C" (Math|Transform|MakeTransform (Variables|Default|GetDemonAimTransform) (Math|Rotator|MakeRotator 0.0 0.0 (Math|Random|RandomFloatinRange -55.0 55.0)) "1.000000,1.000000,1.000000") "AlwaysSpawn" "MultiplyWithRoot" 0 0))
  (Development|PrintString (Utilities|GetDisplayName _returnvalue)))

(event Custom|Tutorialization
  ;[0.15 0.15 0.15 0.5 90] TUTORIAL
  (if (== (Variables|Default|GetStage) 0)
    (CallFunction|TutorialDemonShoot)
    (Utilities|Time|SetGlobalTimeDilation 0.67)
    (Variables|/Script/Engine.Actor|SetCustomTimeDilation (Game|GetPlayerCharacter 0) (/ 1.0 (Class|GameplayStatics|GetGlobalTimeDilation)))
    (elif (== (Variables|Default|GetStage) 1)
      (CallFunction|Stage1))))

(event Custom|TutorialDemonShoot
  ;[0.15 0.15 0.15 0.5 90] TUTORIAL
  (if (and (== (Variables|Default|GetTutorialBulletsFired) 0) (== (Variables|Default|GetTutorialBulletsCaptured) 0))
    (Game|SpawnActorfromClass "/Game/Final/BP_FinalBulletTutorial.BP_FinalBulletTutorial_C" (Math|Transform|MakeTransform (Variables|Default|GetDemonAimTransform) "0.000000,14.000000,0.000000" "1.000000,1.000000,1.000000") "AlwaysSpawn" "MultiplyWithRoot" 0 0)
    (Utilities|FlowControl|Delay 1.0)
    (Math|Integer|IncrementInt (Variables|Default|GetTutorialBulletsFired)
      (:%20%20
        (if (and (== (Variables|Default|GetTutorialBulletsFired) 1) (== (Variables|Default|GetTutorialBulletsCaptured) 1)) :!label _label
          (Game|SpawnActorfromClass "/Game/Final/BP_FinalBulletTutorial.BP_FinalBulletTutorial_C" (Math|Transform|MakeTransform (Variables|Default|GetDemonAimTransform) "0.000000,-25.000000,0.000000" "1.000000,1.000000,1.000000") "AlwaysSpawn" "MultiplyWithRoot" 0 0)
          (Utilities|FlowControl|Delay 1.0)
          (Math|Integer|IncrementInt (Variables|Default|GetTutorialBulletsFired)
            (:%20%20
              (if (and (== (Variables|Default|GetTutorialBulletsFired) 2) (== (Variables|Default|GetTutorialBulletsCaptured) 2)) :!label _label_2
                (Game|SpawnActorfromClass "/Game/Final/BP_FinalBulletTutorial.BP_FinalBulletTutorial_C" (Math|Transform|MakeTransform (Variables|Default|GetDemonAimTransform) "0.000000,48.000000,0.000000" "1.000000,1.000000,1.000000") "AlwaysSpawn" "MultiplyWithRoot" 0 0)
                (Utilities|FlowControl|Delay 1.0)
                (Math|Integer|IncrementInt (Variables|Default|GetTutorialBulletsFired)
                  (:%20%20
                    (if (and (== (Variables|Default|GetTutorialBulletsFired) 3) (== (Variables|Default|GetTutorialBulletsCaptured) 3)) :!label _label_3
                      (Game|SpawnActorfromClass "/Game/Final/BP_FinalBulletTutorial.BP_FinalBulletTutorial_C" (Math|Transform|MakeTransform (Variables|Default|GetDemonAimTransform) "0.000000,48.000000,0.000000" "1.000000,1.000000,1.000000") "AlwaysSpawn" "MultiplyWithRoot" 0 0)
                      (Utilities|FlowControl|Delay 1.0)
                      (Math|Integer|IncrementInt (Variables|Default|GetTutorialBulletsFired)
                        (:%20%20
                          (if (and (== (Variables|Default|GetTutorialBulletsFired) 4) (== (Variables|Default|GetTutorialBulletsCaptured) 4)) :!label _label_4
                            (Game|SpawnActorfromClass "/Game/Final/BP_FinalBulletTutorial.BP_FinalBulletTutorial_C" (Math|Transform|MakeTransform (Variables|Default|GetDemonAimTransform) "0.000000,48.000000,0.000000" "1.000000,1.000000,1.000000") "AlwaysSpawn" "MultiplyWithRoot" 0 0)
                            (Utilities|FlowControl|Delay 1.0)
                            (Math|Integer|IncrementInt (Variables|Default|GetTutorialBulletsFired)
                              (:%20%20
                                (if (and (== (Variables|Default|GetTutorialBulletsFired) 5) (== (Variables|Default|GetTutorialBulletsCaptured) 5)) :!label _label_5
                                  (Game|SpawnActorfromClass "/Game/Final/BP_FinalBulletTutorial.BP_FinalBulletTutorial_C" (Math|Transform|MakeTransform (Variables|Default|GetDemonAimTransform) "0.000000,48.000000,0.000000" "1.000000,1.000000,1.000000") "AlwaysSpawn" "MultiplyWithRoot" 0 0)
                                  (Utilities|FlowControl|Delay 1.0)
                                  (Math|Integer|IncrementInt (Variables|Default|GetTutorialBulletsFired)
                                    (:%20%20
                                      (if (and (== (Variables|Default|GetTutorialBulletsFired) 6) (== (Variables|Default|GetTutorialBulletsCaptured) 6)) :!label _label_6
                                        (Game|SpawnActorfromClass "/Game/Final/BP_FinalBulletTutorial.BP_FinalBulletTutorial_C" (Math|Transform|MakeTransform (Variables|Default|GetDemonAimTransform) "0.000000,48.000000,0.000000" "1.000000,1.000000,1.000000") "AlwaysSpawn" "MultiplyWithRoot" 0 0)
                                        (Utilities|FlowControl|Delay 1.0)
                                        (Math|Integer|IncrementInt (Variables|Default|GetTutorialBulletsFired)
                                          (:%20%20
                                            (if (and (== (Variables|Default|GetTutorialBulletsFired) 7) (== (Variables|Default|GetTutorialBulletsCaptured) 7)) :!label _label_7
                                              (Game|SpawnActorfromClass "/Game/Final/BP_FinalBulletTutorial.BP_FinalBulletTutorial_C" (Math|Transform|MakeTransform (Variables|Default|GetDemonAimTransform) "0.000000,48.000000,0.000000" "1.000000,1.000000,1.000000") "AlwaysSpawn" "MultiplyWithRoot" 0 0)
                                              (Utilities|FlowControl|Delay 1.0)
                                              (Math|Integer|IncrementInt (Variables|Default|GetTutorialBulletsFired)
                                                (:%20%20
                                                  (bind _returnvalue (Actor|GetActorOfClass "/Game/Final/BP_FinalBoss.BP_FinalBoss_C"))
                                                  (Utilities|FlowControl|Delay 2.3)
                                                  (Default|TutorialQTE _returnvalue)
                                                  (Utilities|FlowControl|Delay 2.0)
                                                  (Math|Integer|IncrementInt (Variables|Default|GetStage)
                                                    (:%20%20
                                                      (CallFunction|Stage1)))))
                                              (else
                                                (Utilities|FlowControl|Delay 0.5)
                                                (goto _label_7)))))
                                        (else
                                          (Utilities|FlowControl|Delay 0.5)
                                          (goto _label_6)))))
                                  (else
                                    (Utilities|FlowControl|Delay 0.5)
                                    (goto _label_5)))))
                            (else
                              (Utilities|FlowControl|Delay 0.5)
                              (goto _label_4)))))
                      (else
                        (Utilities|FlowControl|Delay 0.5)
                        (goto _label_3)))))
                (else
                  (Utilities|FlowControl|Delay 0.5)
                  (goto _label_2)))))
          (else
            (Utilities|FlowControl|Delay 0.5)
            (goto _label)))))))

(event Custom|Stage1
  ;[0.15 0.15 0.15 0.5 100] STAGE 1
  (Development|PrintString "Stage 1")
  (if (== (Variables|Default|GetStage) 1)
    (Utilities|Time|SetGlobalTimeDilation 1.0)
    (Variables|/Script/Engine.Actor|SetCustomTimeDilation (Game|GetPlayerCharacter 0) 1.0)
    (Utilities|FlowControl|Sequence
      (:then_0
        (Utilities|FlowControl|Delay 1.4)
        (CallFunction|DemonShoot)
        (Utilities|FlowControl|Delay 1.2)
        (CallFunction|DemonShoot)
        (Utilities|FlowControl|Delay 0.8)
        (CallFunction|DemonShoot)
        (Utilities|FlowControl|Delay 0.67)
        (CallFunction|DemonShoot))
      (:then_1
        (bind _returnvalue (Actor|GetActorOfClass "/Game/Final/BP_FinalBoss.BP_FinalBoss_C"))
        (Utilities|FlowControl|Delay 6.7)
        (Default|StartPreProgrammedQTE _returnvalue)
        (Utilities|FlowControl|Delay 3.45)
        (CallFunction|DemonShoot)))))

(event EventBeginPlay
  (Variables|Default|SetStage 0)
  (bind _asbp_final_player (Utilities|Casting|CastToBP_FinalPlayer (Game|Player|GetPlayerPawn 0)))
  (bind _output_get (Variables|/Game/Final/BP_FinalPlayer.BP_FinalPlayer_C|SetCloseCam _asbp_final_player (Variables|Default|GetCloseCam)))
  (if _output_get
    _
    (else
      ;[0.15 0.15 0.15 0.5 90] Declare Variables
      (bind _returnvalue (Actor|GetActorOfClass "/Script/CinematicCamera.CineCameraActor"))
      (bind _output_get_2 (Variables|Default|SetCamera _returnvalue))
      (Game|Player|SetViewTargetwithBlend (Game|GetPlayerController 0) _output_get_2 0.0 "VTBlend_Linear" 0.0 false)))
  (bind _returnvalue_2 (Actor|GetActorOfClass "/Game/Final/BP_FinalBoss.BP_FinalBoss_C"))
  (bind _output_get_3 (Variables|Default|SetDemon _returnvalue_2))
  (Utilities|IsValid _output_get_3
    (:Is%20Valid
      (Variables|Default|SetDemonAimTransform (Math|Vector|MakeVector (+ (.X (Math|Vector|BreakVector (.location (Transformation|GetActorTransform _output_get_3)))) 1e+02) (.Y (Math|Vector|BreakVector (.location (Transformation|GetActorTransform _output_get_3)))) (.Z (Math|Vector|BreakVector (.location (Transformation|GetActorTransform _output_get_3))))))
      (bind _asbp_final_player_2 (Utilities|Casting|CastToBP_FinalPlayer (Game|GetPlayerCharacter 0)))
      (Variables|/Game/Final/BP_FinalPlayer.BP_FinalPlayer_C|SetPlayerCurrentHealth _asbp_final_player_2 (Variables|/Game/Final/BP_FinalPlayer.BP_FinalPlayer_C|GetPlayerMaxHealth _asbp_final_player_2))
      (CallFunction|Tutorialization))))

(fn ConstructionScript)