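; Final boss actor that runs button-mash grab QTEs against the player and can heal itself, updating the HUD health bar.
; QTE events drop the Forcefield's collision; player presence in GrabZone activates the widget, and mash input fills progress that drains on Tick.
; Tutorial timeout displaces the player and restores the forcefield, while standard timeout just resets.
; A completed mash fires both tutorial-finish and failure handlers, with no separate success path.
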(event OnComponentBeginOverlap(GrabZone)
  (params (OverlappedComponent :type Primitive%20Component%20Object%20Reference) (OtherActor :type Actor%20Object%20Reference) (OtherComp :type Primitive%20Component%20Object%20Reference) (OtherBodyIndex :type Integer) (bFromSweep :type Boolean) (SweepResult :type Hit%20Result%20Structure%20%28by%20ref%29))
  (Variables|/Game/Final/BP_FinalPlayer.BP_FinalPlayer_C|SetInteractableDemon (.AsBP%20Final%20Player (Utilities|Casting|CastToBP_FinalPlayer (Game|GetPlayerCharacter 0))) self)
  (if (not (Variables|Default|GetbIsQTEActive))
    (if (Variables|Default|GetbIsQTEWindowOpen)
      (Variables|Default|SetbIsQTEActive true)
      (Rendering|SetVisibility (Variables|Default|GetWidget) true false))))

(event OnComponentEndOverlap(GrabZone)
  (params (OverlappedComponent :type Primitive%20Component%20Object%20Reference) (OtherActor :type Actor%20Object%20Reference) (OtherComp :type Primitive%20Component%20Object%20Reference) (OtherBodyIndex :type Integer))
  (Variables|/Game/Final/BP_FinalPlayer.BP_FinalPlayer_C|SetInteractableDemon (.AsBP%20Final%20Player (Utilities|Casting|CastToBP_FinalPlayer (Game|GetPlayerCharacter 0))) 0))

(event Custom|Healboss
  (params (HealAmount :type Float%20%28double-precision%29))
  ;[0.15 0.15 0.15 0.5] add damage health logic here
  (Variables|Default|SetBossHealth (+ (Variables|Default|GetBossHealth) HealAmount))
  (bind _asbp_final_player (Utilities|Casting|CastToBP_FinalPlayer (Game|Player|GetPlayerPawn 0)))
  (Default|HealthGainBoss (Variables|/Game/Widget/WBP_Debug.WBP_Debug_C|GetWBP_BossHpBar (Variables|/Game/Final/BP_FinalPlayer.BP_FinalPlayer_C|GetHUD _asbp_final_player))))

(event Custom|ReceiveButtonMash
  (if (Variables|Default|GetbIsQTEActive)
    (bind _output_get (Variables|Default|SetQTE_Progress (Math|Float|Clamp(Float) (+ (Variables|Default|GetQTE_Progress) 0.1))))
    (if (>= (Math|Float|Clamp(Float) (+ (Variables|Default|GetQTE_Progress) 0.1)) 1.0)
      (Development|PrintString (Utilities|String|Append "QTE Progress: " (Utilities|String|ToString(Float) _output_get)))
      (Utilities|Time|ClearandInvalidateTimerbyHandle (Variables|Default|GetQTE_TimerHandle))
      (Variables|Default|SetbIsQTEActive false)
      (Rendering|SetVisibility (Variables|Default|GetWidget) false false)
      (Variables|Default|SetbIsQTEWindowOpen false)
      (Utilities|FlowControl|Sequence
        (:then_0
          (CallFunction|TutorialQTEFinish))
        (:then_1
          (CallFunction|QTEFailed)))
      (else
        (Development|PrintString (Utilities|String|Append "QTE Progress: " (Utilities|String|ToString(Float) _output_get)))))))

(event Custom|StartPreProgrammedQTE
  (Development|PrintString "qte" true false "(R=1.000000,G=0.000000,B=0.645259,A=1.000000)")
  (Variables|Default|SetbIsQTEWindowOpen true)
  (Collision|SetCollisionEnabled (Variables|Default|GetForcefield) "NoCollision")
  (if (Collision|IsOverlappingActor (Variables|Default|GetGrabZone) (Game|GetPlayerCharacter 0) :!class /Script/Engine.PrimitiveComponent)
    (Variables|Default|SetbIsQTEActive true)
    (Rendering|SetVisibility (Variables|Default|GetWidget) true false)
    (bind _returnvalue (Utilities|Time|SetTimerbyEvent (delegate Custom|QTEFailed) 4.0))
    (Variables|Default|SetQTE_TimerHandle _returnvalue)))

(event Custom|TutorialQTE
  (bind _forcefield (Variables|Default|GetForcefield))
  (Development|PrintString "tutorial qte" true false "(R=1.000000,G=0.000000,B=0.645259,A=1.000000)")
  (Variables|Default|SetbIsQTEWindowOpen true)
  (Collision|SetCollisionEnabled _forcefield "NoCollision")
  (Rendering|SetVisibility _forcefield false false)
  (if (Collision|IsOverlappingActor (Variables|Default|GetGrabZone) (Game|GetPlayerCharacter 0) :!class /Script/Engine.PrimitiveComponent)
    (Variables|Default|SetbIsQTEActive true)
    (Rendering|SetVisibility (Variables|Default|GetWidget) true false)
    (bind _returnvalue (Utilities|Time|SetTimerbyEvent (delegate Custom|TutorialQTEFinish) 4.0))
    (Variables|Default|SetQTE_TimerHandle _returnvalue)))

(event Custom|TutorialQTEFinish
  (bind _forcefield (Variables|Default|GetForcefield))
  (Variables|Default|SetbIsQTEActive false)
  (Variables|Default|SetbIsQTEWindowOpen false)
  (Variables|Default|SetQTE_Progress 0.0)
  (Rendering|SetVisibility (Variables|Default|GetWidget) false false)
  (Class|Actor|AddActorWorldTransform (Game|GetPlayerCharacter 0) (Math|Transform|MakeTransform (+ (* (Transformation|GetActorForwardVector self) "1500.000000,1.000000,1.000000") "400.000000,0.000000,30.000000") "0, 0, 0" "1.000000,1.000000,1.000000") true false)
  (Utilities|FlowControl|Delay 0.2)
  (Collision|SetCollisionEnabled _forcefield "QueryAndPhysics")
  (Rendering|SetVisibility _forcefield true false)
  (Development|PrintString "tutorial qte success" true false "(R=1.000000,G=0.000000,B=0.645259,A=1.000000)"))

(event Custom|QTEFailed
  (Variables|Default|SetbIsQTEActive false)
  (Variables|Default|SetbIsQTEWindowOpen false)
  (Variables|Default|SetQTE_Progress 0.0)
  (Rendering|SetVisibility (Variables|Default|GetWidget) false false)
  (Collision|SetCollisionEnabled (Variables|Default|GetForcefield) "QueryAndPhysics"))

(event EventBeginPlay)

(event Collision|EventActorBeginOverlap
  (params (OtherActor :type Actor%20Object%20Reference)))

(event EventTick
  (params (DeltaSeconds :type Float%20%28single-precision%29))
  (if (Variables|Default|GetbIsQTEActive)
    (Variables|Default|SetQTE_Progress (Math|Float|Clamp(Float) (- (Variables|Default|GetQTE_Progress) (* DeltaSeconds (Variables|Default|GetQTE_DrainRate)))))))

(fn ConstructionScript)