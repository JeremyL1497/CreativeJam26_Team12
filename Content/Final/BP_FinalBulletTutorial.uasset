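; Tutorial bullet projectile that the player can catch within reach radius.
; Tick moves it forward at a Timeline-blended speed and feeds position and direction to a particle trail, with target and lifetime still test values.
; Overlap toggles its widget and the player's CatchableBullet, but begin casts to BP_FinalPlayer and end to MarcelPlayer; body hits only print.
; ExecuteCatch increments the GM_Final capture count, triggers the tutorial demon's shot and destroys the bullet.
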(event OnComponentBeginOverlap(Box)
  (params (OverlappedComponent :type Primitive%20Component%20Object%20Reference) (OtherActor :type Actor%20Object%20Reference) (OtherComp :type Primitive%20Component%20Object%20Reference) (OtherBodyIndex :type Integer) (bFromSweep :type Boolean) (SweepResult :type Hit%20Result%20Structure%20%28by%20ref%29))
  (bind _asbp_final_player (Utilities|Casting|CastToBP_FinalPlayer OtherActor))
  (if (== OtherComp (Variables|/Game/Final/BP_FinalPlayer.BP_FinalPlayer_C|GetReachRadius _asbp_final_player))
    (Development|PrintString "Reach")
    (Rendering|SetVisibility (Variables|Default|GetWidget) true false)
    (Variables|/Game/Final/BP_FinalPlayer.BP_FinalPlayer_C|SetCatchableBullet (.AsBP%20Final%20Player (Utilities|Casting|CastToBP_FinalPlayer (Game|GetPlayerCharacter 0))) self)
    (elif (== OtherComp (Variables|/Script/Engine.Character|GetCapsuleComponent _asbp_final_player))
      (Development|PrintString "Hit"))))

(event OnComponentEndOverlap(Box)
  (params (OverlappedComponent :type Primitive%20Component%20Object%20Reference) (OtherActor :type Actor%20Object%20Reference) (OtherComp :type Primitive%20Component%20Object%20Reference) (OtherBodyIndex :type Integer))
  (bind _asmarcel_player (Utilities|Casting|CastToMarcelPlayer OtherActor))
  (if (== OtherComp (Variables|/Game/Marcel/MarcelPlayer.MarcelPlayer_C|GetReachRadius _asmarcel_player))
    (Rendering|SetVisibility (Variables|Default|GetWidget) false false)
    (Variables|/Game/Marcel/MarcelPlayer.MarcelPlayer_C|SetCatchableBullet (.AsMarcel%20Player (Utilities|Casting|CastToMarcelPlayer (Game|GetPlayerCharacter 0))) 0)))

(event EventExecuteCatch
  (bind _returnvalue (Game|GetGameMode))
  (bind _asgm_final (Utilities|Casting|CastToGM_Final _returnvalue))
  ;[0.15 0.15 0.15 0.5] Capture Success Logic
  (bind _result (Math|Integer|IncrementInt (Variables|/Game/Final/GM_Final.GM_Final_C|GetTutorialBulletsCaptured _asgm_final))
    (:%20%20
      (Development|PrintString (Utilities|String|Append (Utilities|String|ToString(Integer) _result) " tutorial bullet(s) captured"))
      (Default|TutorialDemonShoot _asgm_final)
      (Actor|DestroyActor))))

(event EventTick
  (params (DeltaSeconds :type Float%20%28single-precision%29))
  (bind _bullettrail_0 (Variables|Default|GetBulletTrail_0))
  ;[0.15 0.15 0.15 0.5] Plugin the lifetime of the bullet/time left of the bullet before it reaches the catching location
  (Effects|Components|ParticleSystem|SetFloatParameter (Variables|Default|GetBulletTrail_0) "BulletLifetime" 1.0)
  ;[0.15 0.15 0.15 0.5] Activates the FX
  (Components|Activation|Activate (Variables|Default|GetBulletTrail_0) true)
  ;[0.15 0.15 0.15 0.5] For testing purposes only. We'll need to feed the target location once here. The value must not change or the trail will expand beyond the target location.
  (Effects|Components|ParticleSystem|SetVectorParameter _bullettrail_0 "BulletTrailEnd" (* (Variables|Default|GetTrailDistance) (Math|Vector|Normalize (- (Transformation|GetActorLocation) (Variables|Default|GetLastPosition)))))
  ;[0.15 0.15 0.15 0.5] Feed the bullet position when it's moving
  (Effects|Components|ParticleSystem|SetVectorParameter _bullettrail_0 "Bullet" (Transformation|GetActorLocation))
  (Transformation|AddActorWorldOffset (* DeltaSeconds (Math|Float|Lerp (Variables|Default|GetMaxVelocity) (Variables|Default|GetMinVelocity) (stale EventBeginPlay _alpha)) (Transformation|GetActorForwardVector))))

(event EventBeginPlay
  (Variables|Default|SetStartPOS (Transformation|GetActorLocation))
  (bind _alpha (Timeline|Timeline PlayFromStart)))

(fn ConstructionScript
  (|CallParentFunction))